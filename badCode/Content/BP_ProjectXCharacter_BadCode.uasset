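; Character Blueprint, named as a bad-code version, that builds a typed string one letter at a time and shows it on a text render actor in the level.
; A separate function per letter appends a hardcoded, inconsistently cased character to StringToTest, then calls ChangeText.
; ChangeText scans every TextRenderActor on each call and updates the one whose display name is TEXTENTERED.
; Nothing in this Blueprint calls the letter functions.
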(event `self.ReceiveBeginPlay`
  (`parent.ReceiveBeginPlay`))

(fn `AddA`
  (set `self.StringToTest` (`KismetStringLibrary.Concat_StrStr` (`self.StringToTest`) "a"))
  (`self.ChangeText`))

(fn `Addb`
  (set `self.StringToTest` (`KismetStringLibrary.Concat_StrStr` (`self.StringToTest`) "b"))
  (`self.ChangeText`))

(fn `Addc`
  (set `self.StringToTest` (`KismetStringLibrary.Concat_StrStr` (`self.StringToTest`) "c"))
  (`self.ChangeText`))

(fn `Addd`
  (set `self.StringToTest` (`KismetStringLibrary.Concat_StrStr` (`self.StringToTest`) "d"))
  (`self.ChangeText`))

(fn `AddE`
  (set `self.StringToTest` (`KismetStringLibrary.Concat_StrStr` (`self.StringToTest`) "E"))
  (`self.ChangeText`))

(fn `Addf`
  (set `self.StringToTest` (`KismetStringLibrary.Concat_StrStr` (`self.StringToTest`) "f"))
  (`self.ChangeText`))

(fn `Addg`
  (set `self.StringToTest` (`KismetStringLibrary.Concat_StrStr` (`self.StringToTest`) "g"))
  (`self.ChangeText`))

(fn `Addh`
  (set `self.StringToTest` (`KismetStringLibrary.Concat_StrStr` (`self.StringToTest`) "h"))
  (`self.ChangeText`))

(fn `Addi`
  (set `self.StringToTest` (`KismetStringLibrary.Concat_StrStr` (`self.StringToTest`) "i"))
  (`self.ChangeText`))

(fn `Addj`
  (set `self.StringToTest` (`KismetStringLibrary.Concat_StrStr` (`self.StringToTest`) "j"))
  (`self.ChangeText`))

(fn `Addk`
  (set `self.StringToTest` (`KismetStringLibrary.Concat_StrStr` (`self.StringToTest`) "k"))
  (`self.ChangeText`))

(fn `Addl`
  (set `self.StringToTest` (`KismetStringLibrary.Concat_StrStr` (`self.StringToTest`) "l"))
  (`self.ChangeText`))

(fn `Addm`
  (set `self.StringToTest` (`KismetStringLibrary.Concat_StrStr` (`self.StringToTest`) "m"))
  (`self.ChangeText`))

(fn `Addn`
  (set `self.StringToTest` (`KismetStringLibrary.Concat_StrStr` (`self.StringToTest`) "n"))
  (`self.ChangeText`))

(fn `Addo`
  (set `self.StringToTest` (`KismetStringLibrary.Concat_StrStr` (`self.StringToTest`) "o"))
  (`self.ChangeText`))

(fn `AddP`
  (set `self.StringToTest` (`KismetStringLibrary.Concat_StrStr` (`self.StringToTest`) "p"))
  (`self.ChangeText`))

(fn `Addq`
  (set `self.StringToTest` (`KismetStringLibrary.Concat_StrStr` (`self.StringToTest`) "Q"))
  (`self.ChangeText`))

(fn `AddR`
  (set `self.StringToTest` (`KismetStringLibrary.Concat_StrStr` (`self.StringToTest`) "R"))
  (`self.ChangeText`))

(fn `Adds`
  (set `self.StringToTest` (`KismetStringLibrary.Concat_StrStr` (`self.StringToTest`) "s"))
  (`self.ChangeText`))

(fn `AddT`
  (set `self.StringToTest` (`KismetStringLibrary.Concat_StrStr` (`self.StringToTest`) "T"))
  (`self.ChangeText`))

(fn `Addu`
  (set `self.StringToTest` (`KismetStringLibrary.Concat_StrStr` (`self.StringToTest`) "u"))
  (`self.ChangeText`))

(fn `Addv`
  (set `self.StringToTest` (`KismetStringLibrary.Concat_StrStr` (`self.StringToTest`) "v"))
  (`self.ChangeText`))

(fn `Addw`
  (set `self.StringToTest` (`KismetStringLibrary.Concat_StrStr` (`self.StringToTest`) "w"))
  (`self.ChangeText`))

(fn `Addx`
  (set `self.StringToTest` (`KismetStringLibrary.Concat_StrStr` (`self.StringToTest`) "x"))
  (`self.ChangeText`))

(fn `Addy`
  (set `self.StringToTest` (`KismetStringLibrary.Concat_StrStr` (`self.StringToTest`) "y"))
  (`self.ChangeText`))

(fn `AddZ`
  (set `self.StringToTest` (`KismetStringLibrary.Concat_StrStr` (`self.StringToTest`) "z"))
  (`self.ChangeText`))

(fn `ChangeText`
  (bind _outactors (`GameplayStatics.GetAllActorsOfClass` "/Script/Engine.TextRenderActor"))
  (for _array_element _outactors
    (if (== (`KismetSystemLibrary.GetDisplayName` _array_element) "TEXTENTERED")
      (`TextRenderComponent.K2_SetText` (`TextRenderActor.TextRender` _array_element) (`KismetTextLibrary.Conv_StringToText` (`self.StringToTest`))))))

(fn `UserConstructionScript`
  (`parent.UserConstructionScript`))