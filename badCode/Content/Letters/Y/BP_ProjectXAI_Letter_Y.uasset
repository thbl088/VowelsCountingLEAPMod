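; BP_ProjectXAI_Letter_Y is the letter Y AI character, which adds its letter to a BP_ProjectXCharacter_BadCode when damaged by one.
; BeginPlay binds OnDamaged, which casts the damage causer, calls Addy and prints its test string.
; Death with a valid instigator stops voices and plays an attached death cue where cosmetic events can run.
; A random spotted-vocalization loop and an AddA call are left disconnected.
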(event `/Game/Blueprints/Gameplay/PlayerClasses/BP_ProjectXCharacter.Died`
  (params (Victim :type "Actor Object Reference") (Damage :type "Float (single-precision)") (DamageEvent :type "DamageEvent Structure (by ref)") (EventInstigator :type "Controller Object Reference") (DamageCauser :type "Actor Object Reference") (InstigatorPlayerState :type "PlayerState Object Reference"))
  (`parent.Died` Victim Damage DamageEvent EventInstigator DamageCauser InstigatorPlayerState)
  (`/Engine/EditorBlueprintResources/StandardMacros.IsValid` EventInstigator
    (:`Is Valid`
      (`/Engine/EditorBlueprintResources/StandardMacros.Can Execute Cosmetic Events`
        (:`True`
          (`self.StopAllVoices`)
          (`GameplayStatics.SpawnSoundAttached` "/Game/Audio/AI/Spec/Spec_Die_Cue.Spec_Die_Cue" (`self.RootComponent`) "None" (0.0 0.0 0.0) (struct) "KeepRelativeOffset" false 2.0 1.0 0.0 null null))))))

(event `self.ReceiveBeginPlay`
  (`parent.ReceiveBeginPlay`)
  (add `self.OnTakeAnyDamage` (delegate `OnDamaged`)))

(event `OnDamaged` :!signature `self.OnTakeAnyDamage`
  (params (DamagedActor :type "Actor Object Reference") (Damage :type "Float (double-precision)") (DamageType :type "DamageType Object Reference") (InstigatedBy :type "Controller Object Reference") (DamageCauser :type "Actor Object Reference"))
  (bind _asbp_project_xcharacter_bad_code (cast `/badCode/BP_ProjectXCharacter_BadCode` DamageCauser))
  (`/badCode/BP_ProjectXCharacter_BadCode.Addy` _asbp_project_xcharacter_bad_code)
  (`KismetSystemLibrary.PrintString` (`/badCode/BP_ProjectXCharacter_BadCode.StringToTest` _asbp_project_xcharacter_bad_code)))

(fn `UserConstructionScript`
  (`parent.UserConstructionScript`))